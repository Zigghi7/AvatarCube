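; Deprecated hands-free speech-to-text Blueprint that turns the player's microphone speech into Italian text for an assistant.
; AssistantSubsystem state changes drive it: Listening and WaitingForFollowUp start VAD-enabled capture, while other states cancel or reset it.
; When VAD detects speech end, buffered PCM goes to a non-streaming recognizer, whose accumulated segments are submitted to the subsystem.
; Flags discard stale results, and recognition errors rebuild the recognizer if listening is still expected.
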(event Custom|EV_VAD_SpeechStarted
  (if (Variables|Default|GetbIsRecording)
    (if (not (Variables|Default|GetbIsFinalizingSpeech))
      (Variables|Default|SetbSpeechDetected true)
      (Development|PrintString "VAD: SPEECH DETECTED AND STARTED" true true "(R=0.000000,G=1.000000,B=0.026692,A=1.000000)" 5.0))))

(event Custom|EV_STT_RecognizedSegment
  (params (RecognizedWords :type String))
  (bind _returnvalue (Utilities|String|Trim RecognizedWords))
  (if (not (Variables|Default|GetbDiscardRecognitionResult))
    (if (> (Utilities|String|Len _returnvalue) 0)
      (bind _output_get (Variables|Default|SetAccumulatedText (Utilities|String|Append (Variables|Default|GetAccumulatedText) " " _returnvalue)))
      (Development|PrintString (Utilities|String|Append "STT SEGMENT: " _output_get) true true "(R=0.000000,G=1.000000,B=0.209408,A=1.000000)" 5.0))))

(event Custom|ResetSpeechSession
  (bind _capturablesoundwave (Variables|Default|GetCapturableSoundWave))
  (Variables|Default|SetbPendingAutomaticListen false)
  (Utilities|IsValid _capturablesoundwave
    (:Is%20Valid
      (if (Variables|Default|GetbIsRecording)
        (Class|CapturableSoundWave|StopCapture _capturablesoundwave)
        (Class|StreamingSoundWave|ResetVAD _capturablesoundwave)
        (Class|StreamingSoundWave|ToggleVAD _capturablesoundwave false)
        (CallFunction|FinishResetSpeechSession)
        (else
          (Class|StreamingSoundWave|ResetVAD _capturablesoundwave)
          (Class|StreamingSoundWave|ToggleVAD _capturablesoundwave false)
          (CallFunction|FinishResetSpeechSession))))
    (:Is%20Not%20Valid
      (CallFunction|FinishResetSpeechSession))))

(event Custom|EV_VAD_SpeechEnded
  (if (Variables|Default|GetbIsRecording)
    (if (Variables|Default|GetbSpeechDetected)
      (if (not (Variables|Default|GetbIsFinalizingSpeech))
        (Variables|Default|SetbIsFinalizingSpeech true)
        (Development|PrintString "VAD: SPEECH ENDED" true true "(R=0.000000,G=1.000000,B=0.026692,A=1.000000)" 5.0)
        (CallFunction|FinalizeCurrentUtterance)))))

(event Custom|InitializeSpeechRecognizer
  (if (not (or (Variables|Default|GetbRecognizerReady) (Variables|Default|GetbIsStartingRecognition)))
    (Variables|Default|SetbIsStartingRecognition true)
    (bind _returnvalue (Class|SpeechRecognizer|CreateSpeechRecognizer))
    (bind _output_get (Variables|Default|SetSpeechRecognizer _returnvalue))
    (Class|SpeechRecognizer|SetNonStreamingDefaults _output_get)
    (Class|SpeechRecognizer|SetLanguage _output_get "It")
    (Class|SpeechRecognizer|SetTranslatetoEnglish _output_get false)
    (Class|SpeechRecognizer|SetSuppressBlank _output_get true)
    (Class|SpeechRecognizer|SetSuppressNonSpeechTokens _output_get true)
    (Class|SpeechRecognizer|SetNumOfThreads _output_get)
    (EventDispatchers|AssignOnRecognizedTextSegment _output_get (EventDispatchers|CreateEvent :!event Custom|EV_STT_RecognizedSegment))
    (EventDispatchers|AssignOnRecognitionFinished _output_get (EventDispatchers|CreateEvent :!event Custom|EV_STT_RecognitionFinished))
    (EventDispatchers|AssignOnRecognitionError _output_get (EventDispatchers|CreateEvent :!event Custom|EV_STT_RecognitionError))
    (Class|SpeechRecognizer|StartSpeechRecognition (Variables|Default|GetSpeechRecognizer) (delegate Custom|HandleStartSpeechRecognition))))

(event Custom|HandleStartSpeechRecognition
  (params (bSucceeded :type Boolean))
  (if bSucceeded
    (Variables|Default|SetbIsStartingRecognition false)
    (Variables|Default|SetbRecognizerReady true)
    (Development|PrintString "STT RECOGNIZER READY" true true "(R=0.022386,G=1.000000,B=0.244160,A=1.000000)" 5.0)
    (if (Variables|Default|GetbPendingAutomaticListen)
      (Variables|Default|SetbPendingAutomaticListen false)
      (CallFunction|StartListeningAutomatic)
      (else
        (Variables|Default|SetbIsStartingRecognition false)
        (Variables|Default|SetbRecognizerReady false)
        (Development|PrintString "STT RECOGNIZER START FAILED" true true "(R=1.000000,G=0.000000,B=0.010701,A=1.000000)" 5.0)))))

(event Custom|CancelCurrentCapture
  (Variables|Default|SetbPendingAutomaticListen false)
  (Utilities|IsValid (Variables|Default|GetCapturableSoundWave)
    (:Is%20Valid
      (if (Variables|Default|GetbIsRecording)
        (Class|CapturableSoundWave|StopCapture (Variables|Default|GetCapturableSoundWave))
        (CallFunction|DisableCurrentVAD)
        (else
          (CallFunction|DisableCurrentVAD))))
    (:Is%20Not%20Valid
      (CallFunction|FinishCancelCurrentCapture))))

(event Custom|FinalizeCurrentUtterance
  (bind _returnvalue (Subsystems|GetAssistantSubsystem))
  (bind _returnvalue_2 (Class|AssistantSubsystem|GetCurrentState _returnvalue))
  (Utilities|IsValid (Variables|Default|GetCapturableSoundWave)
    (:Is%20Valid
      (if (Variables|Default|GetbIsRecording)
        (Class|CapturableSoundWave|StopCapture (Variables|Default|GetCapturableSoundWave))
        (Variables|Default|SetbIsRecording false)
        (bind _returnvalue_3 (Class|ImportedSoundWave|GetPCMBufferCopy (Variables|Default|GetCapturableSoundWave)))
        (if (> (Utilities|Array|Length _returnvalue_3) 0)
          (Variables|Default|SetbDiscardRecognitionResult false)
          (Class|SpeechRecognizer|ProcessAudioData (Variables|Default|GetSpeechRecognizer) _returnvalue_3 (Math|Conversions|ToFloat(Integer) (Class|ImportedSoundWave|GetSampleRate (Variables|Default|GetCapturableSoundWave))) (Class|ImportedSoundWave|GetNumberOfChannels (Variables|Default|GetCapturableSoundWave)) true)
          (Development|PrintString "STT: AUDIO SENT TO RECOGNIZER" true true "(R=0.001936,G=1.000000,B=0.060244,A=1.000000)" 5.0)
          (Class|StreamingSoundWave|ResetVAD (Variables|Default|GetCapturableSoundWave))
          (Class|StreamingSoundWave|ToggleVAD (Variables|Default|GetCapturableSoundWave) false)
          (else
            (Variables|Default|SetbIsFinalizingSpeech false)
            (Variables|Default|SetbSpeechDetected false)
            (Variables|Default|SetbDiscardRecognitionResult false)
            (Variables|Default|SetCapturableSoundWave 0)
            (Utilities|FlowControl|Delay 0.2)
            (if (or (Utilities|Enum|Equal(Enum) _returnvalue_2 "Listening") (Utilities|Enum|Equal(Enum) _returnvalue_2 "WaitingForFollowUp"))
              (CallFunction|StartListeningAutomatic))))
        (else
          (Variables|Default|SetbIsFinalizingSpeech false)
          (Variables|Default|SetbSpeechDetected false))))
    (:Is%20Not%20Valid
      (Variables|Default|SetbIsFinalizingSpeech false)
      (Variables|Default|SetbSpeechDetected false))))

(event Custom|RestartListeningIfAllowed
  (bind _returnvalue (Subsystems|GetAssistantSubsystem))
  (bind _returnvalue_2 (Class|AssistantSubsystem|GetCurrentState _returnvalue))
  (Utilities|FlowControl|Delay 0.1)
  (if (or (Utilities|Enum|Equal(Enum) _returnvalue_2 "Listening") (Utilities|Enum|Equal(Enum) _returnvalue_2 "WaitingForFollowUp"))
    (CallFunction|StartListeningAutomatic)))

(event Custom|CompleteRecognitionErrorCleanup
  (bind _capturablesoundwave (Variables|Default|GetCapturableSoundWave))
  (Utilities|IsValid _capturablesoundwave
    (:Is%20Valid
      (Class|StreamingSoundWave|ResetVAD _capturablesoundwave)
      (Class|StreamingSoundWave|ToggleVAD _capturablesoundwave false)
      (CallFunction|ResetStateAfterRecognitionError))
    (:Is%20Not%20Valid
      (CallFunction|ResetStateAfterRecognitionError))))

(event Custom|EV_STT_RecognitionFinished
  (if (Variables|Default|GetbDiscardRecognitionResult)
    (Variables|Default|SetbDiscardRecognitionResult false)
    (Variables|Default|SetbIsFinalizingSpeech false)
    (Variables|Default|SetbSpeechDetected false)
    (Variables|Default|SetbIsRecording false)
    (Variables|Default|SetAccumulatedText "")
    (Variables|Default|SetCapturableSoundWave 0)
    (CallFunction|RestartListeningifAllowed)
    (elif (Utilities|Array|IsEmpty (Utilities|String|Trim (Variables|Default|GetAccumulatedText)))
      (Variables|Default|SetbIsFinalizingSpeech false)
      (Variables|Default|SetbSpeechDetected false)
      (Variables|Default|SetbIsRecording false)
      (Variables|Default|SetAccumulatedText "")
      (Variables|Default|SetCapturableSoundWave 0)
      (Development|PrintString "Nessun testo riconosciuto" true true "(R=1.000000,G=0.000000,B=0.045105,A=1.000000)" 5.0)
      (CallFunction|RestartListeningifAllowed)
      (else
        (Development|PrintString (Utilities|String|Append "STT FINAL: " (Variables|Default|GetAccumulatedText)) true true "(R=0.000000,G=1.000000,B=0.209408,A=1.000000)" 5.0)
        (Variables|Default|SetbIsFinalizingSpeech false)
        (Variables|Default|SetbSpeechDetected false)
        (Variables|Default|SetbDiscardRecognitionResult false)
        (Variables|Default|SetbIsRecording false)
        (Variables|Default|SetCapturableSoundWave 0)
        (Class|AssistantSubsystem|SubmitUserText (Subsystems|GetAssistantSubsystem) (Variables|Default|GetAccumulatedText))
        (Variables|Default|SetAccumulatedText "")))))

(event Custom|ResetStateAfterRecognitionError
  (Variables|Default|SetbIsRecording false)
  (Variables|Default|SetbSpeechDetected false)
  (Variables|Default|SetbIsFinalizingSpeech false)
  (Variables|Default|SetbDiscardRecognitionResult false)
  (Variables|Default|SetbPendingAutomaticListen false)
  (Variables|Default|SetAccumulatedText "")
  (Variables|Default|SetCapturableSoundWave 0)
  (Utilities|IsValid (Variables|Default|GetSpeechRecognizer)
    (:Is%20Valid
      (Class|SpeechRecognizer|StopSpeechRecognition (Variables|Default|GetSpeechRecognizer))
      (Variables|Default|SetbRecognizerReady false)
      (Variables|Default|SetbIsStartingRecognition false)
      (Variables|Default|SetSpeechRecognizer 0)
      (CallFunction|RetryRecognitionAfterError))
    (:Is%20Not%20Valid
      (Variables|Default|SetbRecognizerReady false)
      (Variables|Default|SetbIsStartingRecognition false)
      (Variables|Default|SetSpeechRecognizer 0)
      (CallFunction|RetryRecognitionAfterError))))

(event Custom|RetryRecognitionAfterError
  (bind _returnvalue (Subsystems|GetAssistantSubsystem))
  (bind _returnvalue_2 (Class|AssistantSubsystem|GetCurrentState _returnvalue))
  (if (or (Utilities|Enum|Equal(Enum) _returnvalue_2 "Listening") (Utilities|Enum|Equal(Enum) _returnvalue_2 "WaitingForFollowUp"))
    (Variables|Default|SetbPendingAutomaticListen true)
    (Utilities|FlowControl|Delay 0.5)
    (CallFunction|InitializeSpeechRecognizer)))

(event Custom|DisableCurrentVAD
  (bind _capturablesoundwave (Variables|Default|GetCapturableSoundWave))
  (Utilities|IsValid _capturablesoundwave
    (:Is%20Valid
      (Class|StreamingSoundWave|ResetVAD _capturablesoundwave)
      (Class|StreamingSoundWave|ToggleVAD _capturablesoundwave false)
      (CallFunction|FinishCancelCurrentCapture))
    (:Is%20Not%20Valid
      (CallFunction|FinishCancelCurrentCapture))))

(event Custom|FinishCancelCurrentCapture
  (Variables|Default|SetbIsRecording false)
  (Variables|Default|SetbSpeechDetected false)
  (if (Variables|Default|GetbIsFinalizingSpeech)
    (Variables|Default|SetbDiscardRecognitionResult true)
    (Variables|Default|SetAccumulatedText "")
    (else
      (Variables|Default|SetbDiscardRecognitionResult false)
      (Variables|Default|SetbIsFinalizingSpeech false)
      (Variables|Default|SetAccumulatedText "")
      (Variables|Default|SetCapturableSoundWave 0))))

(event Custom|FinishResetSpeechSession
  (Variables|Default|SetbIsRecording false)
  (Variables|Default|SetbSpeechDetected false)
  (Variables|Default|SetbPendingAutomaticListen false)
  (if (Variables|Default|GetbIsFinalizingSpeech)
    (Variables|Default|SetbDiscardRecognitionResult true)
    (Variables|Default|SetAccumulatedText "")
    (Development|PrintString "STT SESSION RESET - PENDING RESULT WILL BE DISCARDED" true true "(R=0.000000,G=0.660000,B=1.000000,A=1.000000)" 5.0)
    (else
      (Variables|Default|SetbDiscardRecognitionResult false)
      (Variables|Default|SetbIsFinalizingSpeech false)
      (Variables|Default|SetAccumulatedText "")
      (Variables|Default|SetCapturableSoundWave 0)
      (Development|PrintString "STT SESSION RESET" true true "(R=0.000000,G=0.660000,B=1.000000,A=1.000000)" 5.0))))

(event Custom|EndPlayStopRecognizer
  (bind _speechrecognizer (Variables|Default|GetSpeechRecognizer))
  (Variables|Default|SetbIsRecording false)
  (Variables|Default|SetbSpeechDetected false)
  (Variables|Default|SetbIsFinalizingSpeech false)
  (Variables|Default|SetbPendingAutomaticListen false)
  (Utilities|IsValid _speechrecognizer
    (:Is%20Valid
      (Class|SpeechRecognizer|StopSpeechRecognition _speechrecognizer)
      (CallFunction|EndPlayClearReferences))
    (:Is%20Not%20Valid
      (CallFunction|EndPlayClearReferences))))

(event Custom|EndPlayClearReferences
  (Variables|Default|SetCapturableSoundWave 0)
  (Variables|Default|SetSpeechRecognizer 0)
  (Variables|Default|SetAccumulatedText "")
  (Variables|Default|SetbRecognizerReady false)
  (Variables|Default|SetbIsStartingRecognition false)
  (Variables|Default|SetbIsRecording false)
  (Variables|Default|SetbSpeechDetected false)
  (Variables|Default|SetbIsFinalizingSpeech false)
  (Variables|Default|SetbDiscardRecognitionResult false)
  (Variables|Default|SetbPendingAutomaticListen false)
  (Development|PrintString "STT END PLAY CLEANUP" true true "(R=0.000000,G=0.660000,B=1.000000,A=1.000000)" 5.0))

(event Custom|EV_STT_RecognitionError
  (params (ShortErrorMessage :type String) (LongErrorMessage :type String))
  (bind _capturablesoundwave (Variables|Default|GetCapturableSoundWave))
  (Development|PrintString (Utilities|String|Append "STT ERROR: " ShortErrorMessage " | " LongErrorMessage) true true "(R=1.000000,G=0.034807,B=0.000000,A=1.000000)" 5.0)
  (Utilities|IsValid _capturablesoundwave
    (:Is%20Valid
      (if (Variables|Default|GetbIsRecording)
        (Class|CapturableSoundWave|StopCapture _capturablesoundwave)
        (CallFunction|CompleteRecognitionErrorCleanup)
        (else
          (CallFunction|CompleteRecognitionErrorCleanup))))
    (:Is%20Not%20Valid
      (CallFunction|CompleteRecognitionErrorCleanup))))

(event Custom|HandleAssistantStateChanged
  (params (NewState :type EAssistantState%20Enum :default "Idle") (PreviousState :type EAssistantState%20Enum :default "Idle"))
  (switch Utilities|FlowControl|Switch|SwitchonEAssistantState NewState
    (:Idle
      (CallFunction|ResetSpeechSession))
    (:PersonDetected
      (CallFunction|CancelCurrentCapture :!label _label))
    (:Greeting
      (goto _label))
    (:Listening
      (if (Variables|Default|GetbAutomaticListeningEnabled) :!label _label_2
        (CallFunction|StartListeningAutomatic)))
    (:ProcessingSpeech
      (CallFunction|CancelCurrentCapture :!label _label_3))
    (:QueryingAI
      (goto _label_3))
    (:Speaking
      (goto _label_3))
    (:WaitingForFollowUp
      (goto _label_2))
    (:EndingInteraction
      (CallFunction|ResetSpeechSession :!label _label_4))
    (:Error
      (goto _label_4))))

(event Custom|StartListeningAutomatic
  (if (Variables|Default|GetbAutomaticListeningEnabled)
    (switch Utilities|FlowControl|Switch|SwitchonEAssistantState (Class|AssistantSubsystem|GetCurrentState (Subsystems|GetAssistantSubsystem))
      (:Listening
        _)
      (:WaitingForFollowUp
        _))
    (if (Variables|Default|GetbRecognizerReady)
      (if (not (or (Variables|Default|GetbIsRecording) (Variables|Default|GetbIsFinalizingSpeech)))
        (Variables|Default|SetbPendingAutomaticListen false)
        (Variables|Default|SetbDiscardRecognitionResult false)
        (Variables|Default|SetbSpeechDetected false)
        (Variables|Default|SetbIsFinalizingSpeech false)
        (Variables|Default|SetAccumulatedText "")
        (bind _returnvalue (Class|CapturableSoundWave|CreateCapturableSoundWave))
        (Variables|Default|SetCapturableSoundWave _returnvalue)
        (Class|StreamingSoundWave|ToggleVAD (Variables|Default|GetCapturableSoundWave) true)
        (Class|StreamingSoundWave|SetVADMode (Variables|Default|GetCapturableSoundWave) "Aggressive")
        (Class|StreamingSoundWave|SetMinimumSpeechDuration (Variables|Default|GetCapturableSoundWave) (Variables|Default|GetMinimumSpeechDurationMs))
        (Class|StreamingSoundWave|SetSilenceDuration (Variables|Default|GetCapturableSoundWave) (Variables|Default|GetSilenceDurationMs))
        (EventDispatchers|AssignOnSpeechStarted (Variables|Default|GetCapturableSoundWave) (delegate Custom|EV_VAD_SpeechStarted))
        (EventDispatchers|AssignOnSpeechEnded (Variables|Default|GetCapturableSoundWave) (delegate Custom|EV_VAD_SpeechEnded))
        (Variables|Default|SetbIsRecording true)
        (Class|CapturableSoundWave|StartCapture (Variables|Default|GetCapturableSoundWave) (Variables|Default|GetMicrophoneDeviceId))
        (Development|PrintString "AUTO LISTENING STARTED" true true "(R=0.000000,G=0.913259,B=1.000000,A=1.000000)" 5.0))
      (else
        (Variables|Default|SetbPendingAutomaticListen true)
        (if (not (Variables|Default|GetbIsStartingRecognition))
          (CallFunction|InitializeSpeechRecognizer))))))

(event EventBeginPlay
  (EventDispatchers|AssignOnStateChanged (Subsystems|GetAssistantSubsystem) (EventDispatchers|CreateEvent :!event Custom|HandleAssistantStateChanged))
  (CallFunction|InitializeSpeechRecognizer))

(event EventEndPlay
  (params (EndPlayReason :type EEndPlayReason%20Enum :default "Destroyed"))
  (bind _capturablesoundwave (Variables|Default|GetCapturableSoundWave))
  (bind _capturablesoundwave_2 (Variables|Default|GetCapturableSoundWave))
  (Variables|Default|SetbPendingAutomaticListen false)
  (Variables|Default|SetbDiscardRecognitionResult true)
  (Utilities|IsValid (Variables|Default|GetCapturableSoundWave)
    (:Is%20Valid
      (if (Variables|Default|GetbIsRecording)
        (Class|CapturableSoundWave|StopCapture _capturablesoundwave_2)
        (Class|StreamingSoundWave|ResetVAD _capturablesoundwave_2)
        (Class|StreamingSoundWave|ToggleVAD _capturablesoundwave_2 false)
        (else
          (Class|StreamingSoundWave|ResetVAD _capturablesoundwave)
          (Class|StreamingSoundWave|ToggleVAD _capturablesoundwave false)))
      (CallFunction|EndPlayStopRecognizer))
    (:Is%20Not%20Valid
      (CallFunction|EndPlayStopRecognizer))))

(fn ConstructionScript)