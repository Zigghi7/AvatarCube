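; Voice Blueprint for an AI assistant that speaks text through TTS with lip sync on the Vivian MetaHuman.
; Text from AssistantSubsystem goes to AssistantTtsClient, and the returned MP3 bytes are imported at runtime and played as 2D sound.
; The sound's PCM data drives a realistic lip-sync generator shared with Vivian's face AnimBP.
; The subsystem is notified after a duration-based delay, on failure or for empty text.
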(event Custom|OnTtsCompleted_Event
  (params (bSuccess :type Boolean) (AudioBytes :type Array%20of%20Bytes))
  (if bSuccess
    (Class|RuntimeAudioImporterLibrary|ImportAudiofromBuffer (Variables|Default|GetRuntimeAudioImporter) AudioBytes "Mp3")
    (else
      (Variables|Default|SetbIsSpeaking false)
      (Class|AssistantSubsystem|NotifyAssistantFinishedSpeaking (Subsystems|GetAssistantSubsystem)))))

(event Custom|OnAssistantTextReady_Event
  (params (TextToSay :type String))
  (if (Utilities|Array|IsEmpty TextToSay)
    (Class|AssistantSubsystem|NotifyAssistantFinishedSpeaking (Subsystems|GetAssistantSubsystem))
    (else
      (Variables|Default|SetbIsSpeaking true)
      (Class|AssistantTtsClient|SynthesizeText (Variables|Default|GetAssistantTtsClient) TextToSay))))

(event Custom|OnGeneratePCMData_Event
  (params (PCMData :type Array%20of%20Floats%20%28single-precision%29))
  (Class|RealisticMetaHumanLipSyncGenerator|ProcessAudioData (Variables|Default|GetLipSyncGenerator) PCMData 44100 1))

(event Custom|OnTtsError_Event
  (params (ErrorMessage :type String))
  (Development|PrintString ErrorMessage true true "(R=1.000000,G=0.042211,B=0.000000,A=1.000000)" 7.0)
  (Variables|Default|SetbIsSpeaking false)
  (Class|AssistantSubsystem|NotifyAssistantFinishedSpeaking (Subsystems|GetAssistantSubsystem)))

(event Custom|AudioImporter_OnProgress_Event
  (params (Percentage :type Integer)))

(event Custom|AudioImporter_OnResult_Event
  (params (Importer :type Runtime%20Audio%20Importer%20Library%20Object%20Reference) (ImportedSoundWave :type Imported%20Sound%20Wave%20Object%20Reference) (Status :type ERuntimeImportStatus%20Enum :default "SuccessfulImport"))
  (Variables|Default|SetCurrentImportedSoundWave ImportedSoundWave)
  (EventDispatchers|AssignOnGeneratePCMData (Variables|Default|GetCurrentImportedSoundWave) (EventDispatchers|CreateEvent :!event Custom|OnGeneratePCMData_Event))
  (Audio|PlaySound2D (Variables|Default|GetCurrentImportedSoundWave) 1.0 1.0 0.0 0 0)
  (Utilities|FlowControl|Delay (+ (Class|ImportedSoundWave|GetDurationConst (Variables|Default|GetCurrentImportedSoundWave)) 0.2))
  (Class|AssistantSubsystem|NotifyAssistantFinishedSpeaking (Subsystems|GetAssistantSubsystem))
  (Variables|Default|SetbIsSpeaking false)
  (Variables|Default|SetCurrentImportedSoundWave 0))

(event EventBeginPlay
  (bind _returnvalue (Class|RuntimeAudioImporterLibrary|CreateRuntimeAudioImporter))
  (bind _output_get (Variables|Default|SetRuntimeAudioImporter _returnvalue))
  (EventDispatchers|AssignOnProgress _output_get (EventDispatchers|CreateEvent :!event Custom|AudioImporter_OnProgress_Event))
  (EventDispatchers|AssignOnResult _output_get (EventDispatchers|CreateEvent :!event Custom|AudioImporter_OnResult_Event))
  (bind _returnvalue_2 (Game|ConstructObjectfromClass "/Script/AvatarZg.AssistantTtsClient"))
  (bind _output_get_2 (Variables|Default|SetAssistantTtsClient _returnvalue_2))
  (Class|AssistantTtsClient|Configure _output_get_2 (Variables|Default|GetTtsEndpointUrl) 9e+01)
  (EventDispatchers|AssignOnTtsCompleted _output_get_2 (EventDispatchers|CreateEvent :!event Custom|OnTtsCompleted_Event))
  (EventDispatchers|AssignOnTtsError _output_get_2 (EventDispatchers|CreateEvent :!event Custom|OnTtsError_Event))
  (EventDispatchers|AssignOnAssistantTextReady (Subsystems|GetAssistantSubsystem) (EventDispatchers|CreateEvent :!event Custom|OnAssistantTextReady_Event))
  (bind _returnvalue_3 (Class|RealisticMetaHumanLipSyncGenerator|CreateRealisticMetaHumanLipSyncGenerator (Utilities|Struct|MakeRealisticMetaHumanLipSyncConfig "HighlyOptimized")))
  (Variables|Default|SetLipSyncGenerator _returnvalue_3)
  (bind (_result _faceskeletalmesh) (CallFunction|GetFaceSkeletalMeshfromMetahuman))
  (if _result
    (Utilities|FlowControl|Delay 0.2)
    (bind _asabp_vivian_face (Utilities|Casting|CastToABP_Vivian_Face (Components|SkeletalMesh|GetAnimInstance _faceskeletalmesh)))
    (bind _output_get_3 (Variables|Default|SetVivianFaceRef _asabp_vivian_face))
    (Variables|/Game/MetahumanAnimators/ABP_Vivian_Face.ABP_Vivian_Face_C|SetLipSyncGenerator _output_get_3 (Variables|Default|GetLipSyncGenerator))))

(fn ConstructionScript)

(fn GetFaceSkeletalMeshfromMetahuman
  (bind _asbp_vivian (Utilities|Casting|CastToBP_Vivian (Variables|Default|GetMetahumanActor)))
  (return true (Variables|/Game/MetaHumans/Vivian/BP_Vivian.BP_Vivian_C|GetFace _asbp_vivian)))