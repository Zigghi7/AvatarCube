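; UI controller actor for a mall assistant that shows a status widget and a mall map overlay driven by assistant and person-detection events.
; On BeginPlay it creates both widgets and binds to the AssistantSubsystem state change and the C++ person-detection actor's presence events.
; State changes set the status visual and hide the map, except Speaking, which shows it after a delay.
; A looping timer feeds presence progress while idle, and idle refresh flags an unavailable webcam.
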(event Custom|OnStateChanged_Event
  (params (NewState :type EAssistantState%20Enum :default "Idle") (PreviousState :type EAssistantState%20Enum :default "Idle"))
  (bind _statuswidget (Variables|Default|GetStatusWidget))
  (switch Utilities|FlowControl|Switch|SwitchonEAssistantState NewState
    (:Idle
      (Default|SetVisualState _statuswidget "NewEnumerator0")
      (CallFunction|RefreshIdleVisual)
      (Default|HideMap (Variables|Default|GetMapWidget)))
    (:PersonDetected
      (Default|SetVisualState _statuswidget "NewEnumerator1")
      (Default|HideMap (Variables|Default|GetMapWidget)))
    (:Greeting
      (Default|SetVisualState _statuswidget "NewEnumerator2")
      (Default|HideMap (Variables|Default|GetMapWidget)))
    (:Listening
      (Default|SetVisualState _statuswidget "NewEnumerator3")
      (Default|HideMap (Variables|Default|GetMapWidget)))
    (:ProcessingSpeech
      (Default|SetVisualState _statuswidget "NewEnumerator4")
      (Default|HideMap (Variables|Default|GetMapWidget)))
    (:QueryingAI
      (Default|SetVisualState _statuswidget "NewEnumerator4")
      (Default|HideMap (Variables|Default|GetMapWidget)))
    (:Speaking
      (Default|SetVisualState _statuswidget "NewEnumerator5")
      (Utilities|FlowControl|Delay 3.0)
      (Default|ShowMap (Variables|Default|GetMapWidget)))
    (:WaitingForFollowUp
      (Default|SetVisualState _statuswidget "NewEnumerator3")
      (Default|HideMap (Variables|Default|GetMapWidget)))
    (:EndingInteraction
      (Default|SetVisualState _statuswidget "NewEnumerator7")
      (Default|HideMap (Variables|Default|GetMapWidget)))
    (:Error
      (Default|SetVisualState _statuswidget "NewEnumerator6")
      (Default|HideMap (Variables|Default|GetMapWidget)))))

(event Custom|OnRawPresenceChanged_Event
  (params (bPersonDetected :type Boolean))
  (CallFunction|RefreshIdleVisual))

(event Custom|RefreshIdleVisual
  (bind _persondetectionactor (Variables|Default|GetPersonDetectionActor))
  (bind _statuswidget (Variables|Default|GetStatusWidget))
  (if (Variables|/Script/AvatarZg.PersonDetectionActor|GetbCameraRunning _persondetectionactor)
    (if (Variables|/Script/AvatarZg.PersonDetectionActor|GetbWaitingForFreshAbsence _persondetectionactor)
      (Default|SetVisualState _statuswidget "NewEnumerator7")
      (elif (Variables|/Script/AvatarZg.PersonDetectionActor|GetbRawPersonDetected _persondetectionactor)
        (Default|SetVisualState _statuswidget "NewEnumerator1")
        (else
          (Default|SetVisualState _statuswidget "NewEnumerator0"))))
    (else
      (Default|SetVisualState _statuswidget "NewEnumerator6")
      (Variables|/Script/UMG.TextBlock|SetText (Variables|/Game/Widget/WBP_AssistantStatus.WBP_AssistantStatus_C|GetTXT_Status _statuswidget) "Webcam non disponibile"))))

(event Custom|OnPresenceConfirmed_Event
  (Default|SetVisualState (Variables|Default|GetStatusWidget) "NewEnumerator2"))

(event Custom|OnAutomaticInteractionStarted_Event
  (Default|SetVisualState (Variables|Default|GetStatusWidget) "NewEnumerator2"))

(event Custom|OnPresenceRearmed_Event
  (Default|SetVisualState (Variables|Default|GetStatusWidget) "NewEnumerator0"))

(event Custom|UpdatePresenceProgress
  (bind _statuswidget (Variables|Default|GetStatusWidget))
  (bind _persondetectionactor (Variables|Default|GetPersonDetectionActor))
  (if (Math|Boolean|ANDBoolean (Utilities|IsValid _persondetectionactor) (Utilities|IsValid (Variables|Default|GetStatusWidget)) (Utilities|Enum|Equal(Enum) (Class|AssistantSubsystem|GetCurrentState (Subsystems|GetAssistantSubsystem)) "Idle") (Variables|/Script/AvatarZg.PersonDetectionActor|GetbRawPersonDetected (Variables|Default|GetPersonDetectionActor)) (not (Variables|/Script/AvatarZg.PersonDetectionActor|GetbWaitingForFreshAbsence (Variables|Default|GetPersonDetectionActor))))
    (Default|SetVisualState _statuswidget "NewEnumerator1")
    (Default|SetPresenceProgress _statuswidget (Variables|/Script/AvatarZg.PersonDetectionActor|GetPresenceProgress01 _persondetectionactor) (Variables|/Script/AvatarZg.PersonDetectionActor|GetRequiredPresenceDurationSeconds _persondetectionactor))))

(event EventBeginPlay
  (bind _returnvalue (UserInterface|CreateWidget "/Game/Widget/WBP_AssistantStatus.WBP_AssistantStatus_C" (Game|GetPlayerController 0)))
  (bind _output_get (Variables|Default|SetStatusWidget _returnvalue))
  (UserInterface|Viewport|AddtoViewport _output_get 0)
  (bind _returnvalue_2 (UserInterface|CreateWidget "/Game/Widget/WBP_MallMapOverlay.WBP_MallMapOverlay_C" (Game|GetPlayerController 0)))
  (bind _output_get_2 (Variables|Default|SetMapWidget _returnvalue_2))
  (UserInterface|Viewport|AddtoViewport _output_get_2 0)
  (bind _returnvalue_3 (Actor|GetActorOfClass "/Game/PersonDetection/CPP_BP_PersonDetectionActor.CPP_BP_PersonDetectionActor_C"))
  (Variables|Default|SetPersonDetectionActor _returnvalue_3)
  (EventDispatchers|AssignOnStateChanged (Subsystems|GetAssistantSubsystem) (delegate Custom|OnStateChanged_Event))
  (EventDispatchers|AssignOnRawPresenceChanged (Variables|Default|GetPersonDetectionActor) (delegate Custom|OnRawPresenceChanged_Event))
  (EventDispatchers|AssignOnPresenceConfirmed (Variables|Default|GetPersonDetectionActor) (delegate Custom|OnPresenceConfirmed_Event))
  (EventDispatchers|AssignOnAutomaticInteractionStarted (Variables|Default|GetPersonDetectionActor) (delegate Custom|OnAutomaticInteractionStarted_Event))
  (EventDispatchers|AssignOnPresenceRearmed (Variables|Default|GetPersonDetectionActor) (delegate Custom|OnPresenceRearmed_Event))
  (Utilities|Time|SetTimerbyEvent (delegate Custom|UpdatePresenceProgress) 0.2 true))

(fn ConstructionScript)